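; Inventory manager component that stores items as stacks of item instances and handles adding, dropping and using them.
; Adding recursively tops up partial stacks, then creates new instances for the remainder, capped at max stack size.
; Item fragments drive behavior: WorldRepresentation gates dropping as a pickup ahead of the owner, while Usable runs the use and optionally consumes one.
; Adds, drops and consumed uses call the inventory-changed notification.
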(fn `AddItemStack`
  (params (NewItemStack :type "StackInfo Structure"))
  (locals (RemainingCountToAdd :type Integer :default 0))
  (bind (_newitemstack_itemdefinition _newitemstack_count _newitemstack_itemstats) (break `StackInfo` (`local.NewItemStack`)))
  (bind _returnvalue (`KismetMathLibrary.Min` (`/Game/Rougelike/Features/Items/BPFL_ItemUtils.GetMaxStackSize` _newitemstack_itemdefinition) (`local.RemainingCountToAdd`)))
  (bind _remainder (`self.FillLeftoverSpace` NewItemStack_ItemDefinition NewItemStack_Count))
  (bind _output_get (set `local.RemainingCountToAdd` _remainder))
  (while (> _output_get 0)
    (bind _returnvalue_2 (`|GenericCreateObject` "/Script/Rougelike.ItemInstance"))
    (`ItemInstance.Initialize` _returnvalue_2 _newitemstack_itemdefinition _newitemstack_itemstats)
    (`KismetArrayLibrary.Array_Add` (`self.InventoryItems`) (make `ItemStack` _returnvalue_2 _returnvalue))
    (set `local.RemainingCountToAdd` (- (`local.RemainingCountToAdd`) _returnvalue)))
  (`self.OnInventoryChanged`))

(fn `ConsumeItem`
  (params (ItemIndex :type Integer))
  (bind _output (`|GetArrayItem` (`self.InventoryItems`) ItemIndex))
  (bind (_iteminstance _count) (break `ItemStack` _output))
  (if (<= _count 1)
    (`KismetArrayLibrary.Array_Remove` (`self.InventoryItems`) (`local.ItemIndex`))
    (else
      (setmembers `ItemStack` :`StructRef` _output :`Count` (- _count 1)))))

(fn `DropItem`
  (params (ItemIndex :type Integer))
  (returns (Sucess :type Boolean))
  (bind _output (`|GetArrayItem` (`self.InventoryItems`) (`local.ItemIndex`)))
  (bind (_iteminstance _count) (break `ItemStack` _output))
  (bind _returnvalue (`ItemInstance.FindFragmentByClass` (`.ItemInstance` (break `ItemStack` _output)) "/Script/Rougelike.ItemFragment_WorldRepresentation"))
  (if (`KismetArrayLibrary.Array_IsValidIndex` (`self.InventoryItems`) ItemIndex)
    (if (and (`KismetSystemLibrary.IsValid` _returnvalue) (`ItemFragment_WorldRepresentation.bCanBeDropped` _returnvalue))
      (`|SpawnActorFromClass` "/Game/Rougelike/Features/Items/BP_ItemPickup.BP_ItemPickup_C" (`KismetMathLibrary.MakeTransform` (`self.GetDropLocation`)) "Undefined" "MultiplyWithRoot" null (make `StackInfo` (`ItemInstance.ItemDefinition` _iteminstance) _count (`ItemInstance.ItemStats` _iteminstance)) null)
      (`KismetArrayLibrary.Array_Remove` (`self.InventoryItems`) (`local.ItemIndex`))
      (`self.OnInventoryChanged`)
      (return true)
      (else
        (return false)))
    (else
      (return false))))

(fn `FillLeftoverSpace`
  (params (ItemDefinition :type "ItemDefinition Class Reference") (TotalAmount :type Integer))
  (returns (Remainder :type Integer))
  (locals (AmountAdded :type Integer :default 0))
  (bind (_stackindex _found) (`self.FindStackWithLeftoverSpace` ItemDefinition))
  (bind _output (`|GetArrayItem` (`self.InventoryItems`) _stackindex))
  (bind (_iteminstance _count) (break `ItemStack` _output))
  (if (> TotalAmount 0)
    (if _found
      (bind _output_get (set `local.AmountAdded` (`KismetMathLibrary.Min` (- (`/Game/Rougelike/Features/Items/BPFL_ItemUtils.GetMaxStackSize` (`ItemInstance.ItemDefinition` _iteminstance)) _count) (`local.TotalAmount`))))
      (setmembers `ItemStack` :`StructRef` _output :`Count` (+ _output_get _count))
      (bind _remainder (`self.FillLeftoverSpace` (`local.ItemDefinition`) (- (`local.TotalAmount`) (`local.AmountAdded`))))
      (return _remainder)
      (else
        (return (`local.TotalAmount`))))
    (else
      (return 0))))

(fn `FindStackWithLeftoverSpace`
  (params (Item :type "ItemDefinition Class Reference"))
  (returns (StackIndex :type Integer) (Found :type Boolean))
  (bind _item (`local.Item`))
  (for (_array_element _array_index) (`self.InventoryItems`)
    (if (and (== (`ItemInstance.ItemDefinition` (break `ItemStack` _array_element)) _item) (< (`.Count` (break `ItemStack` _array_element)) (`/Game/Rougelike/Features/Items/BPFL_ItemUtils.GetMaxStackSize` _item)))
      (return _array_index true)))
  (return -1 false))

(fn `GetDropLocation`
  (returns (Location :type "Vector Structure"))
  (bind _returnvalue (`self.GetOwner`))
  (return (+ (`Actor.K2_GetActorLocation` _returnvalue) (* (`Actor.GetActorForwardVector` _returnvalue) 200.0))))

(fn `TryUseItem`
  (params (ItemIndex :type Integer))
  (returns (Success :type Boolean))
  (bind _output_iteminstance (break `ItemStack` (`|GetArrayItem` (`self.InventoryItems`) ItemIndex)))
  (bind _returnvalue (`ItemInstance.FindFragmentByClass` _output_iteminstance "/Script/Rougelike.ItemFragment_Usable"))
  (`/Engine/EditorBlueprintResources/StandardMacros.IsValid` _returnvalue
    (:`Is Valid`
      (bind _returnvalue_2 (`ItemFragment_Usable.Use` _returnvalue (`self.GetOwner`)))
      (if (and _returnvalue_2 (`ItemFragment_Usable.bConsumeOnUse` _returnvalue))
        (`self.ConsumeItem` (`local.ItemIndex`))
        (`self.OnInventoryChanged`)
        (return true)
        (else
          (return _returnvalue_2))))))