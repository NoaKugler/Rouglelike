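; BP_Weapon_Base is a base weapon that detects hits and applies a Gameplay Ability System effect to struck pawns.
; HitScanStart stores an effect spec, clears the hit list and starts a looping timer at about 30 Hz; HitScanEnd stops it.
; HitScan sphere-traces between TraceStart and TraceEnd, ignoring the instigator, applying the spec once per target with an ability system component and drawing debug traces.
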(event `HitScan`
  (bind _hitactors (`self.HitActors`))
  (bind _outhits (`KismetSystemLibrary.SphereTraceMultiForObjects` (`SceneComponent.K2_GetComponentLocation` (`self.Trace Start`)) (`SceneComponent.K2_GetComponentLocation` (`self.Trace End`)) (`self.HitScanRadius`) (`|MakeArray` "ObjectTypeQuery3" :!type "EObjectTypeQuery Enum") false (`|MakeArray` (`self.Instigator`) :!type "Actor Object Reference") "ForDuration" true (struct :`R` 1.0 :`A` 1.0) (struct :`G` 1.0 :`A` 1.0) 0.2))
  (for _array_element _outhits
    (bind (_bblockinghit _binitialoverlap _time _distance _location _impactpoint _normal _impactnormal _physmat _hitactor) (`GameplayStatics.BreakHitResult` _array_element))
    (bind _returnvalue (`AbilitySystemBlueprintLibrary.GetAbilitySystemComponent` _hitactor))
    (`/Engine/EditorBlueprintResources/StandardMacros.IsValid` _returnvalue
      (:`Is Valid`
        (if (not (`KismetArrayLibrary.Array_Contains` _hitactors _hitactor))
          (`KismetArrayLibrary.Array_AddUnique` _hitactors _hitactor)
          (`AbilitySystemComponent.BP_ApplyGameplayEffectSpecToSelf` _returnvalue (`self.Effect Spec Handle`)))))))

(event `HitScan Start`
  (params (EffectSpecHandle :type "GameplayEffectSpecHandle Structure"))
  (set `self.Effect Spec Handle` EffectSpecHandle)
  (`KismetArrayLibrary.Array_Clear` (`self.HitActors`))
  (bind _returnvalue (`KismetSystemLibrary.K2_SetTimerDelegate` (`|CreateDelegate` :!event `HitScan`) 0.033333 true))
  (set `self.HitScanTimerHandle` _returnvalue))

(event `HitScan End`
  (`KismetSystemLibrary.K2_ClearAndInvalidateTimerHandle` (`self.HitScanTimerHandle`)))

(fn `UserConstructionScript`)