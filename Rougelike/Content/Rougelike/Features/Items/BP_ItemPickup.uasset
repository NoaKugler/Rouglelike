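; BP_ItemPickup is a world pickup that gives its ItemStack to an overlapping actor that has an inventory.
; On overlap it looks for a BP_InventoryManagerComponent on the other actor, adds the stack to it and destroys itself.
; The construction script sets the static mesh from the item definition's ItemFragment_WorldRepresentation, so the pickup's appearance follows the fragment-based item data.
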(event `self.ReceiveActorBeginOverlap`
  (params (OtherActor :type "Actor Object Reference"))
  (bind _returnvalue (`self.GetComponentByClass` OtherActor "/Game/Rougelike/Features/Inventory/BP_InventoryManagerComponent.BP_InventoryManagerComponent_C"))
  (`/Engine/EditorBlueprintResources/StandardMacros.IsValid` _returnvalue
    (:`Is Valid`
      (`/Game/Rougelike/Features/Inventory/BP_InventoryManagerComponent.AddItemStack` _returnvalue (`self.ItemStack`))
      (`self.K2_DestroyActor`))))

(fn `UserConstructionScript`
  (bind _itemstack_itemdefinition (break `StackInfo` (`self.ItemStack`)))
  (`StaticMeshComponent.SetStaticMesh` (`self.StaticMesh`) (`ItemFragment_WorldRepresentation.ItemMesh` (`ItemDefinition.FindFragmentByClass` _itemstack_itemdefinition "/Script/Rougelike.ItemFragment_WorldRepresentation"))))