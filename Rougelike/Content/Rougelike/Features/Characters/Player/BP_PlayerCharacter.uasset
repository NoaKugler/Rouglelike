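; Player character Blueprint that routes input to Gameplay Ability System abilities, weapon equipping and the inventory menu.
; An attribute listener drives mana regen: a drop removes the regen effect and reapplies it after a short delay, and reaching max removes it.
; Dash activates by class and attack by tag, while hardcoded keys apply a heal or equip sword or staff.
; Inventory toggles via FlipFlop on the UI manager's menu layer.
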(event `self.ReceiveBeginPlay`
  ; Setup
  (bind (_asynctaskproxy _attribute _newvalue _oldvalue) (`AbilityAsync_WaitAttributeChanged.WaitForAttributeChanged` null (struct :`AttributeName` "Mana" :`Attribute` "/Script/Rougelike.CoreAttributeSet:Mana" :`AttributeOwner` "/Script/CoreUObject.Class'/Script/Rougelike.CoreAttributeSet'"))
    (:`Changed`
      (`self.HandleManaChanged` _newvalue _oldvalue))))

(event `HandleManaChanged`
  (params (NewValue :type "Float (double-precision)") (OldValue :type "Float (double-precision)"))
  (bind (_maxmana_basevalue _maxmana_currentvalue) (break `GameplayAttributeData` (`CoreAttributeSet.MaxMana` (`self.CoreAttributeSet`))))
  ; Handle Mana Changed
  (if (< NewValue OldValue)
    (`AbilitySystemComponent.RemoveActiveEffectsWithGrantedTags` (`self.AbilitySystemComponent`) (struct :`GameplayTags` (struct :`(TagName` "Status.Mana.Regen"))))
    (`KismetSystemLibrary.Delay` 1.0)
    (`AbilitySystemComponent.BP_ApplyGameplayEffectToSelf` :`self` (`self.AbilitySystemComponent`) :`GameplayEffectClass` "/Game/Rougelike/Features/GameplayAbilitySystem/Effects/GE_ManaRegen.GE_ManaRegen_C")
    (elif (>= NewValue _maxmana_currentvalue)
      (`AbilitySystemComponent.RemoveActiveEffectsWithGrantedTags` (`self.AbilitySystemComponent`) (struct :`GameplayTags` (struct :`(TagName` "Status.Mana.Regen")))))))

(event `EnhancedInput|/Game/Rougelike/Features/Characters/Player/Input/Actions/IA_Dash`
  (params (ActionValue :type Boolean) (ElapsedSeconds :type "Float (double-precision)") (TriggeredSeconds :type "Float (double-precision)") (InputAction :type "InputAction Object Reference" :default "/Game/Rougelike/Features/Characters/Player/Input/Actions/IA_Dash.IA_Dash"))
  ; Input Action Bindings
  (:`Triggered`
    (`AbilitySystemComponent.TryActivateAbilityByClass` (`self.AbilitySystemComponent`) "/Game/Rougelike/Features/GameplayAbilitySystem/Abilities/Dash/GA_Dash.GA_Dash_C" true)))

(event `Key|H`
  (params (Key :type "Key Structure"))
  ; Input Action Bindings
  (:`Pressed`
    (`AbilitySystemComponent.BP_ApplyGameplayEffectToSelf` :`self` (`self.AbilitySystemComponent`) :`GameplayEffectClass` "/Game/Rougelike/Features/GameplayAbilitySystem/Effects/GE_Heal.GE_Heal_C")))

(event `EnhancedInput|/Game/Rougelike/Features/Characters/Player/Input/Actions/IA_ToggleEquip`
  (params (ActionValue :type Boolean) (ElapsedSeconds :type "Float (double-precision)") (TriggeredSeconds :type "Float (double-precision)") (InputAction :type "InputAction Object Reference" :default "/Game/Rougelike/Features/Characters/Player/Input/Actions/IA_ToggleEquip.IA_ToggleEquip"))
  ; Input Action Bindings
  (:`Triggered`
    (`/Game/Rougelike/Features/Equipment/Weapons/WeaponsManagerComponent.ToggleWeaponEquip` (`self.WeaponsManagerComponent`) "/Game/Rougelike/Features/Equipment/Weapons/Staff/BP_Weapon_Staff.BP_Weapon_Staff_C")))

(event `Key|One`
  (params (Key :type "Key Structure"))
  ; Input Action Bindings
  (:`Pressed`
    (`/Game/Rougelike/Features/Equipment/Weapons/WeaponsManagerComponent.EquipWeapon` (`self.WeaponsManagerComponent`) "/Game/Rougelike/Features/Equipment/Weapons/Sword/BP_Weapon_Sword.BP_Weapon_Sword_C")))

(event `Key|Two`
  (params (Key :type "Key Structure"))
  ; Input Action Bindings
  (:`Pressed`
    (`/Game/Rougelike/Features/Equipment/Weapons/WeaponsManagerComponent.EquipWeapon` (`self.WeaponsManagerComponent`) "/Game/Rougelike/Features/Equipment/Weapons/Staff/BP_Weapon_Staff.BP_Weapon_Staff_C")))

(event `EnhancedInput|/Game/Rougelike/Features/Characters/Player/Input/Actions/IA_Attack`
  (params (ActionValue :type Boolean) (ElapsedSeconds :type "Float (double-precision)") (TriggeredSeconds :type "Float (double-precision)") (InputAction :type "InputAction Object Reference" :default "/Game/Rougelike/Features/Characters/Player/Input/Actions/IA_Attack.IA_Attack"))
  ; Input Action Bindings
  (:`Triggered`
    (`AbilitySystemComponent.TryActivateAbilitiesByTag` (`self.AbilitySystemComponent`) (`BlueprintGameplayTagLibrary.MakeGameplayTagContainerFromArray` (`|MakeArray` (struct :`TagName` "GameplayAbility.Attack") :!type "GameplayTag Structure")) true)))

(event `EnhancedInput|/Game/Rougelike/Features/Characters/Player/Input/Actions/IA_ToggleInventory`
  (params (ActionValue :type Boolean) (ElapsedSeconds :type "Float (double-precision)") (TriggeredSeconds :type "Float (double-precision)") (InputAction :type "InputAction Object Reference" :default "/Game/Rougelike/Features/Characters/Player/Input/Actions/IA_ToggleInventory.IA_ToggleInventory"))
  (bind _returnvalue (subsystem `UIManagerSubsystem`))
  ; Input Action Bindings
  (:`Triggered`
    (`/Engine/EditorBlueprintResources/StandardMacros.FlipFlop`
      (:`A`
        (`UIManagerSubsystem.PushWidget` _returnvalue (struct :`TagName` "UI.Layer.Menu") "/Game/Rougelike/Features/Inventory/UI/WBP_Inventory.WBP_Inventory_C"))
      (:`B`
        (`UIManagerSubsystem.ClearLayer` _returnvalue (struct :`TagName` "UI.Layer.Menu"))))))

(fn `UserConstructionScript`)