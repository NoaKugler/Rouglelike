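; Base enemy Blueprint whose graph displays floating damage numbers when the enemy is damaged.
; HandleDamaged rounds the damage, splits it into characters and spawns one FloatingDamageFX Niagara system per digit at the health bar, using camera yaw and roll for orientation.
; Each system gets its digit texture through a user parameter and is shifted by DigitOffset, which grows per digit and is not reset in this graph.
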(event `self.HandleDamaged`
  (params (DamageAmount :type "Float (single-precision)"))
  (bind (_returnvalue_roll _returnvalue_pitch _returnvalue_yaw) (`KismetMathLibrary.BreakRotator` (`PlayerCameraManager.GetCameraRotation` (`GameplayStatics.GetPlayerCameraManager` 0))))
  (for _array_element (`KismetStringLibrary.GetCharacterArrayFromString` (`KismetStringLibrary.Conv_IntToString` (`KismetMathLibrary.Round` DamageAmount)))
    (bind _returnvalue (`NiagaraFunctionLibrary.SpawnSystemAtLocation` "/Game/Rougelike/Features/GameplayAbilitySystem/VFX/FloatingDamage/FloatingDamageFX.FloatingDamageFX" (`SceneComponent.K2_GetComponentLocation` (`self.HealthBarComponent`)) (`KismetMathLibrary.MakeRotator` _returnvalue_roll 180.0 _returnvalue_yaw)))
    (bind _output_get (set `self.DigitSystem` _returnvalue))
    (`SceneComponent.K2_AddLocalOffset` _output_get (`KismetMathLibrary.MakeVector` 0.0 (`self.DigitOffset`)) false false)
    (set `self.DigitOffset` (+ (`self.DigitOffset`) 25.0))
    (switch `string` _array_element
      (:`0`
        (`NiagaraFunctionLibrary.SetTextureObject` (`self.DigitSystem`) "user.DamageDigit" "/Game/Rougelike/Features/GameplayAbilitySystem/VFX/FloatingDamage/DigitTextures/0.0"))
      (:`1`
        (`NiagaraFunctionLibrary.SetTextureObject` (`self.DigitSystem`) "user.DamageDigit" "/Game/Rougelike/Features/GameplayAbilitySystem/VFX/FloatingDamage/DigitTextures/1.1"))
      (:`2`
        (`NiagaraFunctionLibrary.SetTextureObject` (`self.DigitSystem`) "user.DamageDigit" "/Game/Rougelike/Features/GameplayAbilitySystem/VFX/FloatingDamage/DigitTextures/2.2"))
      (:`3`
        (`NiagaraFunctionLibrary.SetTextureObject` (`self.DigitSystem`) "user.DamageDigit" "/Game/Rougelike/Features/GameplayAbilitySystem/VFX/FloatingDamage/DigitTextures/3.3"))
      (:`4`
        (`NiagaraFunctionLibrary.SetTextureObject` (`self.DigitSystem`) "user.DamageDigit" "/Game/Rougelike/Features/GameplayAbilitySystem/VFX/FloatingDamage/DigitTextures/4.4"))
      (:`5`
        (`NiagaraFunctionLibrary.SetTextureObject` (`self.DigitSystem`) "user.DamageDigit" "/Game/Rougelike/Features/GameplayAbilitySystem/VFX/FloatingDamage/DigitTextures/5.5"))
      (:`6`
        (`NiagaraFunctionLibrary.SetTextureObject` (`self.DigitSystem`) "user.DamageDigit" "/Game/Rougelike/Features/GameplayAbilitySystem/VFX/FloatingDamage/DigitTextures/6.6"))
      (:`7`
        (`NiagaraFunctionLibrary.SetTextureObject` (`self.DigitSystem`) "user.DamageDigit" "/Game/Rougelike/Features/GameplayAbilitySystem/VFX/FloatingDamage/DigitTextures/7.7"))
      (:`8`
        (`NiagaraFunctionLibrary.SetTextureObject` (`self.DigitSystem`) "user.DamageDigit" "/Game/Rougelike/Features/GameplayAbilitySystem/VFX/FloatingDamage/DigitTextures/8.8"))
      (:`9`
        (`NiagaraFunctionLibrary.SetTextureObject` (`self.DigitSystem`) "user.DamageDigit" "/Game/Rougelike/Features/GameplayAbilitySystem/VFX/FloatingDamage/DigitTextures/9.9")))))

(fn `UserConstructionScript`)