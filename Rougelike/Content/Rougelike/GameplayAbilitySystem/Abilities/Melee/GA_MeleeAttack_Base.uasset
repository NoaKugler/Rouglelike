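; Base melee attack gameplay ability that plays a montage and drives the equipped weapon's hit scan.
; On activation it gets the weapon from the avatar's WeaponsManagerComponent and ends if weapon or montage is invalid.
; On authority only, gameplay events start the scan with an outgoing hit effect spec and stop it.
; Montage exit ends the ability, ability end also stops scanning, and OnMontageStarted is an empty override hook.
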(event `self.K2_ActivateAbility`
  (bind _returnvalue (`Actor.GetComponentByClass` (`self.GetAvatarActorFromActorInfo`) "/Game/Rougelike/Weapons/WeaponsManagerComponent.WeaponsManagerComponent_C"))
  (`/Engine/EditorBlueprintResources/StandardMacros.IsValid` _returnvalue
    (:`Is Valid`
      (bind _equippedweapon (`/Game/Rougelike/Weapons/WeaponsManagerComponent.EquippedWeapon` _returnvalue)
        (:`then`
          (set `self.Equipped Weapon` _equippedweapon)
          (bind _montage_to_play (`self.Montage to Play`)
            (:`then`
              (`AbilityTask_PlayMontageAndWait.CreatePlayMontageAndWaitProxy` "None" _montage_to_play 1.0 "None" true 1.0 0.0 true
                (:`then`
                  (`self.OnMontageStarted`)
                  (`self.K2_HasAuthority`
                    (:`True`
                      (`AbilityTask_WaitGameplayEvent.WaitGameplayEvent` (struct :`TagName` "Event.HitScan.Start") null
                        (:`then`
                          (`AbilityTask_WaitGameplayEvent.WaitGameplayEvent` (struct :`TagName` "Event.HitScan.End") null
                            (:`EventReceived`
                              (`self.HandleHitScanEnd`))))
                        (:`EventReceived`
                          (`self.HandleHitScanStart`))))))
                (:`OnCompleted`
                  (`self.K2_EndAbility` :!label _label))
                (:`OnInterrupted`
                  (goto _label))
                (:`OnCancelled`
                  (goto _label))))
            (:`else`
              (`self.K2_EndAbility` :!label _label_2))))
        (:`else`
          (goto _label_2))))
    (:`Is Not Valid`
      (goto _label_2))))

(event `OnMontageStarted`
  ; Empty, Ready for Override
)

(event `self.K2_OnEndAbility`
  (params (bWasCancelled :type Boolean))
  (`self.HandleHitScanEnd`))

(fn `HandleHitScanEnd`
  (bind _equipped_weapon (`self.Equipped Weapon`)
    (:`then`
      (`/Game/Rougelike/Weapons/BP_Weapon_Base.HitScan End` _equipped_weapon))
    (:`else`)))

(fn `HandleHitScanStart`
  (bind _equipped_weapon (`self.Equipped Weapon`)
    (:`then`
      (`/Game/Rougelike/Weapons/BP_Weapon_Base.HitScan Start` _equipped_weapon (`self.MakeOutgoingGameplayEffectSpec` (`self.HitEffectClass`))))
    (:`else`)))